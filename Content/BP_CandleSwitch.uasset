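; BP_CandleSwitch is a switch actor that responds to the player character's Candle state through a custom event.
; If Candle is set on BP_ThirdPersonCharacter, a timeline rolls the candle mesh component by its float track times Angle.
; The sequence's second branch calls DestroyActor immediately, regardless of that check and without waiting for the timeline to finish.
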(event Custom|CustomEvent
  (Utilities|FlowControl|Sequence
    (:then_0
      (bind _asbp_third_person_character (Utilities|Casting|CastToBP_ThirdPersonCharacter (Game|GetPlayerCharacter 0)))
      (if (Variables|/Game/ThirdPerson/Blueprints/BP_ThirdPersonCharacter.BP_ThirdPersonCharacter_C|Getcandle%20 _asbp_third_person_character)
        (bind _float (Timeline|Timeline Play)
          (:Update
            (Transformation|SetRelativeRotation (Variables|Default|Getcandle_StaticMeshComponent1) (Math|Rotator|MakeRotator (* _float (Variables|Default|GetAngle)) 0.0 0.0) false false)))))
    (:then_1
      (Actor|DestroyActor))))

(event EventBeginPlay)

(event Collision|EventActorBeginOverlap
  (params (OtherActor :type Actor%20Object%20Reference)))

(event EventTick
  (params (DeltaSeconds :type Float%20%28single-precision%29)))

(fn ConstructionScript)